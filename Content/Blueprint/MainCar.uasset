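; Player car Blueprint with flashing lights, a sheep-moving siren, health, and game-over screens.
; Looping timers drive FlipFlops for alternating lights and input-held turn signals, while brake input shows two other lights.
; The siren toggle, when switched on, messages tagged sheep inside Box1 to move, and Box overlaps damage the car.
; BeginPlay adds health and 120-second countdown widgets; zero health, the dead event and pause input show paused-game menus.
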(event OnComponentBeginOverlap(Box)
  (params (OverlappedComponent :type Primitive%20Component%20Object%20Reference) (OtherActor :type Actor%20Object%20Reference) (OtherComp :type Primitive%20Component%20Object%20Reference) (OtherBodyIndex :type Integer) (bFromSweep :type Boolean) (SweepResult :type Hit%20Result%20Structure%20%28by%20ref%29))
  (Game|Damage|ApplyDamage self 1e+01 0 OtherActor))

(event Custom|ToogleRight
  ;[1 1 1] ToggleLightCligno
  (Utilities|FlowControl|FlipFlop
    (:A
      (Development|SetHiddeninGame (Variables|Default|GetPointLight4) true false))
    (:B
      (Development|SetHiddeninGame (Variables|Default|GetPointLight4) false false))))

(event Custom|dead
  (bind _returnvalue (UserInterface|CreateWidget "/Game/Widget/Lose.Lose_C"))
  (UserInterface|Viewport|AddtoViewport _returnvalue 0)
  (Variables|/Script/Engine.PlayerController|SetbShowMouseCursor (Game|GetPlayerController 0) true)
  (Game|SetGamePaused true))

(event Custom|ChangeLights
  ;[1 1 1] FunctionCallToggleLight
  (Utilities|FlowControl|FlipFlop
    (:A
      (Development|SetHiddeninGame (Variables|Default|GetPointLight1) true false)
      (Development|SetHiddeninGame (Variables|Default|GetPointLight) false false))
    (:B
      (Development|SetHiddeninGame (Variables|Default|GetPointLight1) false false)
      (Development|SetHiddeninGame (Variables|Default|GetPointLight) true false))))

(event Custom|ToogleLeft
  ;[1 1 1] ToggleLightCligno
  (Utilities|FlowControl|FlipFlop
    (:A
      (Development|SetHiddeninGame (Variables|Default|GetPointLight5) true false))
    (:B
      (Development|SetHiddeninGame (Variables|Default|GetPointLight5) false false))))

(event Input|EnhancedActionEvents|EnhancedInputActionSheep
  (params (ActionValue :type Boolean) (ElapsedSeconds :type Float%20%28double-precision%29) (TriggeredSeconds :type Float%20%28double-precision%29) (InputAction :type Input%20Action%20Object%20Reference :default "/Game/Sheep.Sheep"))
  (:Started
    ;[1 1 1] Sirène
    (if (Variables|Default|GetIsSoundPlaying)
      (Audio|Components|Audio|Stop (Variables|Default|GetAudioCurveSource))
      (Variables|Default|SetIsSoundPlaying false)
      (else
        (Audio|Components|Audio|Play (Variables|Default|GetAudioCurveSource) 0.0)
        (Variables|Default|SetIsSoundPlaying true)
        (for _array_element (Collision|GetOverlappingActors (Variables|Default|GetBox1) "/Game/Blueprint/Sheep.Sheep_C" :!class /Script/Engine.PrimitiveComponent)
          (if (Actor|ActorHasTag _array_element "Interact")
            (Class|CarInterface|MoveSheep(Message) _array_element)))))))

(event Input|EnhancedActionEvents|EnhancedInputActionPause
  (params (ActionValue :type Boolean) (ElapsedSeconds :type Float%20%28double-precision%29) (TriggeredSeconds :type Float%20%28double-precision%29) (InputAction :type Input%20Action%20Object%20Reference :default "/Game/Pause.Pause"))
  ;[1 1 1] Pause
  (bind _asvehicle_adv_game_mode (Utilities|Casting|CastToVehicleAdvGameMode (Game|GetGameMode)))
  (Variables|/Game/VehicleTemplate/Blueprints/VehicleAdvGameMode.VehicleAdvGameMode_C|SetPlay _asvehicle_adv_game_mode false)
  (if (not (Variables|Default|GetPause?))
    (bind _returnvalue (UserInterface|CreateWidget "/Game/Widget/Pause.Pause_C" (Game|GetPlayerController 0)))
    (bind _output_get (Variables|Default|SetPauseWidget _returnvalue))
    (UserInterface|Viewport|AddtoViewport _output_get 0)
    (Game|SetGamePaused true)))

(event Game|Damage|EventAnyDamage
  (params (Damage :type Float%20%28single-precision%29) (DamageType :type Damage%20Type%20Object%20Reference) (InstigatedBy :type Controller%20Object%20Reference) (DamageCauser :type Actor%20Object%20Reference))
  (Variables|Default|SetHealth (- (Variables|Default|GetHealth) Damage))
  (if (<= (Variables|Default|GetHealth) 0.0)
    (bind _returnvalue (UserInterface|CreateWidget "/Game/Widget/Dead.Dead_C"))
    (UserInterface|Viewport|AddtoViewport _returnvalue 0)
    (Variables|/Script/Engine.PlayerController|SetbShowMouseCursor (Game|GetPlayerController 0) true)
    (Game|SetGamePaused true)))

(event EventBeginPlay
  (Utilities|Time|SetTimerbyFunctionName self "ChangeLights" 0.5 true)
  (bind _returnvalue (UserInterface|CreateWidget "/Game/Widget/HealthBar.HealthBar_C"))
  (bind _output_get (Variables|Default|SetHealthUI _returnvalue))
  (UserInterface|Viewport|AddtoViewport _output_get 0)
  (bind _returnvalue_2 (UserInterface|CreateWidget "/Game/Widget/CountDown.CountDown_C"))
  (bind _output_get_2 (Variables|Default|SetCountDown _returnvalue_2))
  (UserInterface|Viewport|AddtoViewport _output_get_2 0))

(event Input|GamepadEvents|GamepadLeftStickLeft
  (params (Key :type Key%20Structure :default "None"))
  (:Pressed
    (Utilities|Time|SetTimerbyFunctionName 0 "ToogleLeft" 0.5 true))
  (:Released
    (Utilities|Time|ClearTimerbyFunctionName 0 "ToogleLeft")
    (Development|SetHiddeninGame (Variables|Default|GetPointLight5) true false)))

(event Input|KeyboardEvents|D
  (params (Key :type Key%20Structure :default "None"))
  (:Pressed
    (Utilities|Time|SetTimerbyFunctionName 0 "ToogleRight" 0.5 true))
  (:Released
    (Utilities|Time|ClearTimerbyFunctionName 0 "ToogleRight")
    (Development|SetHiddeninGame (Variables|Default|GetPointLight4) true false)))

(event Input|KeyboardEvents|Q
  (params (Key :type Key%20Structure :default "None"))
  (:Pressed
    (Utilities|Time|SetTimerbyFunctionName 0 "ToogleLeft" 0.5 true))
  (:Released
    (Utilities|Time|ClearTimerbyFunctionName 0 "ToogleLeft")
    (Development|SetHiddeninGame (Variables|Default|GetPointLight5) true false)))

(event Input|GamepadEvents|GamepadLeftStickRight
  (params (Key :type Key%20Structure :default "None"))
  (:Pressed
    (Utilities|Time|SetTimerbyFunctionName 0 "ToogleRight" 0.5 true))
  (:Released
    (Utilities|Time|ClearTimerbyFunctionName 0 "ToogleRight")
    (Development|SetHiddeninGame (Variables|Default|GetPointLight4) true false)))

(event Input|KeyboardEvents|S
  (params (Key :type Key%20Structure :default "None"))
  (:Pressed
    (Development|SetHiddeninGame (Variables|Default|GetPointLight2) false false)
    (Development|SetHiddeninGame (Variables|Default|GetPointLight3) false false))
  (:Released
    (Development|SetHiddeninGame (Variables|Default|GetPointLight2) true false)
    (Development|SetHiddeninGame (Variables|Default|GetPointLight3) true false)))

(event Input|GamepadEvents|GamepadLeftTriggerAxis
  (params (Key :type Key%20Structure :default "None"))
  (:Pressed
    (Development|SetHiddeninGame (Variables|Default|GetPointLight2) false false)
    (Development|SetHiddeninGame (Variables|Default|GetPointLight3) false false))
  (:Released
    (Development|SetHiddeninGame (Variables|Default|GetPointLight2) true false)
    (Development|SetHiddeninGame (Variables|Default|GetPointLight3) true false)))

(fn ConstructionScript)